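; Main menu character-select actor that displays a customizable character, loaded through its CharacterCustomizer component on BeginPlay and, with authority, during construction.
; Construction picks the Character or SkeletalMesh component as attach root, hides the other, and creates its dynamic materials.
; It adds tagged apparel, hair and groom components per customizer type, linking skeletal parts via master pose.
; Events toggle cloth physics through the customizer.
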(event `self.ReceiveBeginPlay`
  (`/Game/CharacterCustomizer/Character_Customizer/Data/CharacterCustomizer.Load` (`self.CharacterCustomizer`)))

(event `Event Disable Cloth`
  ;[0.2842 0.5625 0.3483] Enable/disable cloth physics
  (`/Game/CharacterCustomizer/Character_Customizer/Data/CharacterCustomizer.Disable Cloth` (`self.CharacterCustomizer`)))

(event `Event Enable Cloth`
  ;[0.2842 0.5625 0.3483] Enable/disable cloth physics
  (`/Game/CharacterCustomizer/Character_Customizer/Data/CharacterCustomizer.Enable Cloth` (`self.CharacterCustomizer`)))

(fn `UserConstructionScript`
  (locals (Attach :type "SkeletalMeshComponent Object Reference"))
  (bind _character (`self.Character`))
  (bind _attach (`local.Attach`))
  (bind _skeletalmesh (`self.SkeletalMesh`))
  (`/Engine/EditorBlueprintResources/StandardMacros.IsValid` (`SkinnedMeshComponent.SkeletalMesh` (`self.SkeletalMesh`))
    (:`Is Valid`
      ;[1 1 1] Character skel mesh will be used for attachment and visuals if valid
      (`/Engine/EditorBlueprintResources/StandardMacros.IsValid` (`SkinnedMeshComponent.SkeletalMesh` (`self.Character`))
        (:`Is Valid`
          (set `local.Attach` _character)
          (`SceneComponent.SetHiddenInGame` _skeletalmesh true false))
        (:`Is Not Valid`
          (set `local.Attach` _skeletalmesh)
          (`SceneComponent.SetHiddenInGame` _character true false)))
      (`|ExecutionSequence`
        (:`then_0`
          ;[1 1 1] Create Material Instances
          (for (_ _array_index) (`MeshComponent.GetMaterials` _attach)
            (bind _returnvalue (`PrimitiveComponent.CreateDynamicMaterialInstance` _attach _array_index null "None"))
            (`KismetArrayLibrary.Array_Set` (`/Game/CharacterCustomizer/Character_Customizer/Data/CharacterCustomizer.Character Materials` (`self.CharacterCustomizer`)) _array_index _returnvalue true)))
        (:`then_1`
          ;[1 1 1] Add apparel mesh components
          (for _array_element (`/Game/CharacterCustomizer/Character_Customizer/Data/CharacterCustomizer.Apparel Types` (`self.CharacterCustomizer`))
            (bind _returnvalue_2 (`AddComponent|NODE_AddCC_SkelMeshComponent-1` :`bManualAttachment` true))
            (`SceneComponent.K2_AttachToComponent` _returnvalue_2 (`local.Attach`) "None" "SnapToTarget" "SnapToTarget" "SnapToTarget" true)
            (set `ActorComponent.ComponentTags` (`|MakeArray` "Apparel" (`KismetStringLibrary.Conv_StringToName` (`|GetEnumeratorNameAsString` _array_element))) _returnvalue_2)))
        (:`then_2`
          ;[1 1 1] Add hair mesh components
          (for _array_element_2 (`/Game/CharacterCustomizer/Character_Customizer/Data/CharacterCustomizer.Hair Types` (`self.CharacterCustomizer`))
            (bind _returnvalue_3 (`AddComponent|NODE_AddCC_SkelMeshComponent-0` :`bManualAttachment` true))
            (`SceneComponent.K2_AttachToComponent` _returnvalue_3 (`local.Attach`) "None" "SnapToTarget" "SnapToTarget" "SnapToTarget" true)
            (bind _returnvalue_4 (`|GetEnumeratorNameAsString` _array_element_2))
            (set `ActorComponent.ComponentTags` (`|MakeArray` (`KismetStringLibrary.Conv_StringToName` _returnvalue_4) "Hair Component") _returnvalue_3)
            ;[1 1 1] Add Groom components
            (bind _returnvalue_5 (`AddComponent|NODE_AddGroomComponent-0` :`bManualAttachment` true))
            (`ActorComponent.SetTickGroup` _returnvalue_5 "TG_PostUpdateWork")
            (`SceneComponent.K2_AttachToComponent` _returnvalue_5 (`local.Attach`) "None" "SnapToTarget" "SnapToTarget" "SnapToTarget" false)
            (set `ActorComponent.ComponentTags` (`|MakeArray` (`KismetStringLibrary.Conv_StringToName` (`KismetTextLibrary.Conv_TextToString` (`|FormatText` "{Name} Groom" _returnvalue_4))) "Hair Component") _returnvalue_5)))
        (:`then_3`
          ;[1 1 1] Load in viewport (disable if networked)
          (`/Engine/EditorBlueprintResources/ActorMacros.Switch Has Authority`
            (:`Authority`
              (`/Game/CharacterCustomizer/Character_Customizer/Data/CharacterCustomizer.Load` (`self.CharacterCustomizer`)))))
        (:`then_4`)
        (:`then_5`
          ;[1 1 1] Set MPC (for editor only)
          (for _array_element_3 (`self.K2_GetComponentsByClass` "/Game/CharacterCustomizer/Character_Customizer/Data/CC_SkelMeshComponent.CC_SkelMeshComponent_C")
            (`SkinnedMeshComponent.SetLeaderPoseComponent` _array_element_3 (`local.Attach`) true)))))))