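; Main menu preview character that displays a customizable male or female avatar through its CharacterCustomizer component, loading it on BeginPlay or on a refresh event.
; SetFemale and SetMale close the customizer menu, swap both skeletal meshes with single-node idle animations, set gender and default profile, then reload and open the apparel menu.
; The U key flip-flops between both genders, while customizer and dresser interaction snippets remain unconnected.
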(event `self.ReceiveBeginPlay`
  (`/Game/CharacterCustomizer/Character_Customizer/Data/CharacterCustomizer.Load` (`self.CharacterCustomizer`) :!label _label))

(event `Refresh Characterr`
  (goto _label))

(event `SetFemale`
  (bind _charactercustomizer (`self.CharacterCustomizer`))
  (bind _character (`self.Character`))
  (bind _mesh (`self.Mesh`))
  (`/Game/CharacterCustomizer/Character_Customizer/Data/CharacterCustomizer.Close Menu` (`self.GetCharacterCustomizer`) false :!label _label_2)
  (`SkeletalMeshComponent.SetAnimationMode` _character "AnimationSingleNode")
  (`SkeletalMeshComponent.SetAnimation` _character "/Game/CharacterCustomizer/Character_Customizer/Characters/Animations/Animations/Idle/Idle.Idle")
  (`SkinnedMeshComponent.SetSkinnedAssetAndUpdate` _character "/Game/CharacterCustomizer/Character_Customizer/Characters/CC_Human/CC_Female.CC_Female" true)
  (`SkinnedMeshComponent.SetSkinnedAssetAndUpdate` _mesh "/Game/CharacterCustomizer/Character_Customizer/Characters/CC_Human/CC_Female_AnimMesh.CC_Female_AnimMesh" true)
  (`SkeletalMeshComponent.SetAnimationMode` _mesh "AnimationSingleNode")
  (`SkeletalMeshComponent.SetAnimation` _mesh "/Game/CharacterCustomizer/Character_Customizer/Characters/Animations/Poses/Pose_Idle_01.Pose_Idle_01")
  (set `self.GetCharacterCustomizer` (`self.CharacterCustomizer`))
  (set `/Game/CharacterCustomizer/Character_Customizer/Data/CharacterCustomizer.Character Name` "F_Default" _charactercustomizer)
  (set `/Game/CharacterCustomizer/Character_Customizer/Data/CharacterCustomizer.Default Character Name` "F_Default" _charactercustomizer)
  (set `/Game/CharacterCustomizer/Character_Customizer/Data/CharacterCustomizer.IsFemale` true _charactercustomizer)
  (`/Game/CharacterCustomizer/Character_Customizer/Data/CharacterCustomizer.Load` _charactercustomizer :!label _label_3)
  (`/Game/CharacterCustomizer/Character_Customizer/Data/CharacterCustomizer.Create Apparel Menu` (`self.CharacterCustomizer`)))

(event `Key|U`
  (params (Key :type "Key Structure"))
  (bind _character (`self.Character`))
  (bind _mesh (`self.Mesh`))
  (bind _charactercustomizer (`self.CharacterCustomizer`))
  (:`Pressed`
    (`/Engine/EditorBlueprintResources/StandardMacros.FlipFlop`
      (:`A`
        (goto _label_2))
      (:`B`
        (`/Game/CharacterCustomizer/Character_Customizer/Data/CharacterCustomizer.Close Menu` (`self.GetCharacterCustomizer`) false :!label _label_4)
        (`SkeletalMeshComponent.SetAnimationMode` _character "AnimationSingleNode")
        (`SkeletalMeshComponent.SetAnimation` _character "/Game/CharacterCustomizer/Character_Customizer/Characters/Animations/Animations/Idle/Idle.Idle")
        (`SkinnedMeshComponent.SetSkinnedAssetAndUpdate` _character "/Game/CharacterCustomizer/Character_Customizer/Characters/CC_Human/CC_Male.CC_Male" true)
        (`SkinnedMeshComponent.SetSkinnedAssetAndUpdate` _mesh "/Game/CharacterCustomizer/Character_Customizer/Characters/CC_Human/CC_Male_AnimMesh.CC_Male_AnimMesh" true)
        (`SkeletalMeshComponent.SetAnimationMode` _mesh "AnimationSingleNode")
        (`SkeletalMeshComponent.SetAnimation` _mesh "/Game/CharacterCustomizer/Character_Customizer/Characters/Animations/Animations/Idle/Idle.Idle")
        (set `self.GetCharacterCustomizer` (`self.CharacterCustomizer`))
        (set `/Game/CharacterCustomizer/Character_Customizer/Data/CharacterCustomizer.Character Name` "M_Default" _charactercustomizer)
        (set `/Game/CharacterCustomizer/Character_Customizer/Data/CharacterCustomizer.Default Character Name` "M_Default" _charactercustomizer)
        (set `/Game/CharacterCustomizer/Character_Customizer/Data/CharacterCustomizer.IsFemale` false _charactercustomizer)
        (goto _label_3)))))

(event `Set Male`
  (goto _label_4))

(fn `UserConstructionScript`
  (`parent.UserConstructionScript`))