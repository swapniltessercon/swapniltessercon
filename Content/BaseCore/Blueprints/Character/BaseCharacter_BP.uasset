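; Base character Blueprint for a modular customization system, building body, apparel and hair from its CharacterCustomizer component.
; The Construction Script picks Character or Mesh as attach parent, creates dynamic materials, and spawns tagged apparel, hair and groom components plus a hidden-in-game name label.
; Modular skeletal parts follow the parent through master pose.
; CharacterCustomizer.Load applies the character on BeginPlay, refresh events and authority-side construction for viewport preview.
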(event `self.ReceiveBeginPlay`
  (`/Game/CharacterCustomizer/Character_Customizer/Data/CharacterCustomizer.Load` (`self.CharacterCustomizer`) :!label _label))

(event `Refresh Characterr`
  (goto _label))

(event `Key|H`
  (params (Key :type "Key Structure"))
  ;[0.126 1 0.07761] Development only keybindings
  (:`Pressed`
    (bind _foundwidgets (`WidgetBlueprintLibrary.GetAllWidgetsOfClass` "/Game/CharacterCustomizer/Character_Customizer/UMG/Keybinds.Keybinds_C"))
    (bind _output (`|GetArrayItem` _foundwidgets))
    (`/Engine/EditorBlueprintResources/StandardMacros.IsValid` _output
      (:`Is Valid`
        (`/Game/CharacterCustomizer/Character_Customizer/UMG/Keybinds.Hide` _output)))))

(event `Key|Alt+MouseScrollUp`
  (params (Key :type "Key Structure"))
  ;[0.126 1 0.07761] Development only keybindings
  (:`Pressed`
    (bind _returnvalue (`GameplayStatics.GetActorOfClass` null))))

(event `Key|Alt+MouseScrollDown`
  (params (Key :type "Key Structure"))
  ;[0.126 1 0.07761] Development only keybindings
  (:`Pressed`
    (bind _returnvalue (`GameplayStatics.GetActorOfClass` null))))

(event `CustomEvent`
  (params (Hide :type Boolean))
  ;[0 0 0] This function should be implemented on the child blueprint (see CC_Character_Full)
)

(event `CustomEvent_1`
  ;[0 0 0] Refresh character in viewport
  (`/Game/CharacterCustomizer/Character_Customizer/Data/CharacterCustomizer.Load` (`self.CharacterCustomizer`)))

(fn `UserConstructionScript`
  (locals (Attach :type "SkeletalMeshComponent Object Reference"))
  (bind _mesh (`self.Mesh`))
  (bind _character (`self.Character`))
  (bind _attach (`local.Attach`))
  (`/Engine/EditorBlueprintResources/StandardMacros.IsValid` (`SkinnedMeshComponent.SkeletalMesh` (`self.Mesh`))
    (:`Is Valid`
      ;[1 1 1] Character skel mesh will be used for attachment and visuals if valid
      (`/Engine/EditorBlueprintResources/StandardMacros.IsValid` (`SkinnedMeshComponent.SkeletalMesh` (`self.Character`))
        (:`Is Valid`
          (set `local.Attach` _character)
          (`SceneComponent.SetHiddenInGame` _mesh true false))
        (:`Is Not Valid`
          (set `local.Attach` _mesh)
          (`SceneComponent.SetHiddenInGame` _character true false)))
      (`|ExecutionSequence`
        (:`then_0`
          ;[1 1 1] Create Material Instances
          (for (_ _array_index) (`MeshComponent.GetMaterials` _attach)
            (bind _returnvalue (`PrimitiveComponent.CreateDynamicMaterialInstance` _attach _array_index null "None"))
            (`KismetArrayLibrary.Array_Set` (`/Game/CharacterCustomizer/Character_Customizer/Data/CharacterCustomizer.Character Materials` (`self.CharacterCustomizer`)) _array_index _returnvalue true)))
        (:`then_1`
          ;[1 1 1] Add apparel mesh components
          (for _array_element (`/Game/CharacterCustomizer/Character_Customizer/Data/CharacterCustomizer.Apparel Types` (`self.CharacterCustomizer`))
            (bind _returnvalue_2 (`AddComponent|NODE_AddCC_SkelMeshComponent-1` :`bManualAttachment` true))
            (`SceneComponent.K2_AttachToComponent` _returnvalue_2 (`local.Attach`) "None" "SnapToTarget" "SnapToTarget" "SnapToTarget" true)
            (set `ActorComponent.ComponentTags` (`|MakeArray` "Apparel" (`KismetStringLibrary.Conv_StringToName` (`|GetEnumeratorNameAsString` _array_element))) _returnvalue_2)))
        (:`then_2`
          ;[1 1 1] Add hair mesh components
          (for _array_element_2 (`/Game/CharacterCustomizer/Character_Customizer/Data/CharacterCustomizer.Hair Types` (`self.CharacterCustomizer`))
            (bind _returnvalue_3 (`AddComponent|NODE_AddCC_SkelMeshComponent-0` :`bManualAttachment` true))
            (`SceneComponent.K2_AttachToComponent` _returnvalue_3 (`local.Attach`) "None" "SnapToTarget" "SnapToTarget" "SnapToTarget" true)
            (bind _returnvalue_4 (`|GetEnumeratorNameAsString` _array_element_2))
            (set `ActorComponent.ComponentTags` (`|MakeArray` (`KismetStringLibrary.Conv_StringToName` _returnvalue_4) "Hair Component") _returnvalue_3)
            ;[1 1 1] Add Groom components
            (bind _returnvalue_5 (`AddComponent|NODE_AddGroomComponent-0` :`bManualAttachment` true))
            (`ActorComponent.SetTickGroup` _returnvalue_5 "TG_PostUpdateWork")
            (`SceneComponent.K2_AttachToComponent` _returnvalue_5 (`local.Attach`) "None" "SnapToTarget" "SnapToTarget" "SnapToTarget" false)
            (set `ActorComponent.ComponentTags` (`|MakeArray` (`KismetStringLibrary.Conv_StringToName` (`KismetTextLibrary.Conv_TextToString` (`|FormatText` "{Name} Groom" _returnvalue_4))) "Hair Component") _returnvalue_5)))
        (:`then_3`
          ;[1 1 1] Load in viewport (disable if networked)
          (`/Engine/EditorBlueprintResources/ActorMacros.Switch Has Authority`
            (:`Authority`
              (`/Game/CharacterCustomizer/Character_Customizer/Data/CharacterCustomizer.Load` (`self.CharacterCustomizer`)))))
        (:`then_4`
          ;[1 1 1] Add name text component
          (bind _returnvalue_6 (`AddComponent|NODE_AddTextRenderComponent-0` :`RelativeTransform` (`KismetMathLibrary.MakeTransform` (`KismetMathLibrary.MakeVector` 0.0 0.0 (+ (`CapsuleComponent.CapsuleHalfHeight` (`self.CapsuleComponent`)) 10.0)))))
          (`PrimitiveComponent.SetMaterial` _returnvalue_6 0 "/Game/CharacterCustomizer/Misc_Materials/M_Text_PlayerFacing.M_Text_PlayerFacing")
          (`TextRenderComponent.SetHorizontalAlignment` _returnvalue_6 "EHTA_Center")
          (`TextRenderComponent.K2_SetText` _returnvalue_6 (`KismetTextLibrary.Conv_NameToText` (`/Game/CharacterCustomizer/Character_Customizer/Data/CharacterCustomizer.Character Name` (`self.CharacterCustomizer`))))
          (`SceneComponent.SetHiddenInGame` _returnvalue_6 true false)
          (`SceneComponent.SetAbsolute` _returnvalue_6 false true false))
        (:`then_5`
          ;[1 1 1] Set MPC (for editor only)
          (for _array_element_3 (`self.K2_GetComponentsByClass` "/Game/CharacterCustomizer/Character_Customizer/Data/CC_SkelMeshComponent.CC_SkelMeshComponent_C")
            (`SkinnedMeshComponent.SetLeaderPoseComponent` _array_element_3 (`local.Attach`) true)))))))