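; Tessercon character Blueprint that loads its customized look through the CharacterCustomizer component.
; BeginPlay and the RefreshCharacterr event both call CharacterCustomizer.Load, the only live logic here.
; The construction script's entry is unwired, so its setup graph never runs.
; That dormant graph creates dynamic materials, tagged apparel, hair and groom components, and a name label, then loads on authority and sets master pose for editor preview.
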(event `self.ReceiveBeginPlay`
  (`/Game/CharacterCustomizer/Character_Customizer/Data/CharacterCustomizer.Load` (`self.CharacterCustomizer`) :!label _label))

(event `Refresh Characterr`
  (goto _label))

(fn `UserConstructionScript`)